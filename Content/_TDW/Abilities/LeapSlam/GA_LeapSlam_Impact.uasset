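; GA_LeapSlam_Impact is a gameplay ability for the impact of a leap slam, hitting actors within an emanation area.
; On activation it commits, gathers the actors in the emanation, runs SlamActor on each, then ends.
; SlamActor knocks each actor away from the emanation origin with velocity override, then applies the ability's effects to that actor's ability system component.
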(event `self.K2_ActivateAbility`
  (bind _returnvalue (`self.K2_CommitAbility`))
  (if _returnvalue
    (bind _outactors (`self.GetActorsInEmanation`))
    (for _array_element _outactors
      (`self.SlamActor` _array_element)))
  (`self.K2_EndAbility`))

(fn `SlamActor`
  (params (Actor :type "Actor Object Reference"))
  (`self.ApplyKnockback` Actor (`self.GetEmanationOrigin`) true)
  (`self.ApplyEffectsToTaget` (`AbilitySystemBlueprintLibrary.GetAbilitySystemComponent` Actor)))